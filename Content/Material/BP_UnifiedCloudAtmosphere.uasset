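; Planet actor that renders a unified atmosphere and volumetric cloud layer as a raymarched post-process effect.
; The construction script puts dynamic raymarcher and blur-control material instances into the post-process component, forces uniform scale, and splits LightColor into StarLight's intensity and color.
; MaterialHooks pushes scattering, noise, step-count and blur settings to both materials, deriving planet center, radius and light direction from the actor transform.
; Nothing runs at runtime.
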(fn `MaterialHooks`
  (bind _uca_post (`self.UCA_POST`))
  (bind _uca_dmi (`self.UCA_DMI`))
  (bind _x (.x (`self.GetActorRelativeScale3D`)))
  ; Light
  (`MaterialInstanceDynamic.SetVectorParameterValue` _uca_dmi "Light Color" (`self.Light Color`))
  (`MaterialInstanceDynamic.SetVectorParameterValue` _uca_dmi "Light Direction" (`KismetMathLibrary.Conv_VectorToLinearColor` (`self.GetActorForwardVector`)))
  ; Scale and Position
  (`MaterialInstanceDynamic.SetVectorParameterValue` _uca_dmi "Planet Center" (`KismetMathLibrary.Conv_VectorToLinearColor` (`self.K2_GetActorLocation`)))
  (`MaterialInstanceDynamic.SetScalarParameterValue` _uca_dmi "Planet Radius" (.x (`self.GetActorRelativeScale3D`)))
  (`MaterialInstanceDynamic.SetScalarParameterValue` _uca_dmi "Atmosphere Height Scale" (`self.Atmosphere Height Scale`))
  (`MaterialInstanceDynamic.SetScalarParameterValue` _uca_dmi "Cloud Outer Height Scale" (`self.Cloud Outer Height Scale`))
  (`MaterialInstanceDynamic.SetScalarParameterValue` _uca_dmi "Cloud Inner Height Scale" (`self.Cloud Inner Height Scale`))
  (`MaterialInstanceDynamic.SetScalarParameterValue` _uca_dmi "Atmosphere Floor Offset" (`self.Atmosphere Floor Offset`))
  ; Atmo Scattering
  (`MaterialInstanceDynamic.SetVectorParameterValue` _uca_dmi "Rayleigh Beta" (`self.Rayleigh Beta`))
  (`MaterialInstanceDynamic.SetVectorParameterValue` _uca_dmi "Mie Beta" (`self.Mie Beta`))
  (`MaterialInstanceDynamic.SetVectorParameterValue` _uca_dmi "Atmosphere Absorption Beta" (`self.Atmosphere Absorption Beta`))
  (`MaterialInstanceDynamic.SetVectorParameterValue` _uca_dmi "Atmosphere Ambient" (`self.Atmosphere Ambient`))
  (`MaterialInstanceDynamic.SetScalarParameterValue` _uca_dmi "Rayleigh Height" (`self.Rayleigh Height`))
  (`MaterialInstanceDynamic.SetScalarParameterValue` _uca_dmi "Mie Height" (`self.Mie Height`))
  (`MaterialInstanceDynamic.SetScalarParameterValue` _uca_dmi "Mie G" (`self.Mie G`))
  (`MaterialInstanceDynamic.SetScalarParameterValue` _uca_dmi "Atmosphere Absorption Height" (`self.Atmosphere Absorption Height`))
  (`MaterialInstanceDynamic.SetScalarParameterValue` _uca_dmi "Atmosphere Absorption Falloff" (`self.Atmosphere Absorption Falloff`))
  ; Cloud Scattering
  (`MaterialInstanceDynamic.SetVectorParameterValue` _uca_dmi "Cloud Beta" (`self.Cloud Beta`))
  (`MaterialInstanceDynamic.SetVectorParameterValue` _uca_dmi "Cloud Absorption Beta" (`self.Cloud Absorption Beta`))
  (`MaterialInstanceDynamic.SetVectorParameterValue` _uca_dmi "Cloud Ambient" (`self.Cloud Ambient`))
  (`MaterialInstanceDynamic.SetVectorParameterValue` _uca_dmi "Cloud Phase Params" (`self.Cloud Phase Params`))
  ; Cloud Noise Params
  (`MaterialInstanceDynamic.SetTextureParameterValue` _uca_dmi "Cloud Volume Texture" (`self.Cloud Volume Texture`))
  (`MaterialInstanceDynamic.SetVectorParameterValue` _uca_dmi "Cloud Noise Weights" (`self.Cloud Noise Weights`))
  (`MaterialInstanceDynamic.SetVectorParameterValue` _uca_dmi "Cloud Noise Invert" (`self.Cloud Noise Invert`))
  (`MaterialInstanceDynamic.SetVectorParameterValue` _uca_dmi "Detail Noise Weights" (`self.Detail Noise Weights`))
  (`MaterialInstanceDynamic.SetVectorParameterValue` _uca_dmi "Detail Noise Invert" (`self.Detail Noise Invert`))
  (`MaterialInstanceDynamic.SetVectorParameterValue` _uca_dmi "Animation Weights" (`self.Animation Weights`))
  (`MaterialInstanceDynamic.SetScalarParameterValue` _uca_dmi "Cloud Coverage" (`self.Cloud Coverage`))
  (`MaterialInstanceDynamic.SetScalarParameterValue` _uca_dmi "Cloud Density Multiplier" (`self.Cloud Density Multiplier`))
  (`MaterialInstanceDynamic.SetScalarParameterValue` _uca_dmi "Cloud Height Curve Max" (`self.Cloud Height Curve Max`))
  (`MaterialInstanceDynamic.SetScalarParameterValue` _uca_dmi "Cloud Height Curve Min" (`self.Cloud Height Curve Min`))
  (`MaterialInstanceDynamic.SetScalarParameterValue` _uca_dmi "Cloud Noise Frequency" (`self.Cloud Noise Frequency`))
  (`MaterialInstanceDynamic.SetScalarParameterValue` _uca_dmi "Detail Erode Strength" (`self.Detail Erode Strength`))
  (`MaterialInstanceDynamic.SetScalarParameterValue` _uca_dmi "Detail Noise Frequency" (`self.Detail Noise Frequency`))
  ; Raymarching
  (`MaterialInstanceDynamic.SetScalarParameterValue` _uca_dmi "Atmosphere Steps" (`KismetMathLibrary.Conv_IntToDouble` (`self.Atmosphere Steps`)))
  (`MaterialInstanceDynamic.SetScalarParameterValue` _uca_dmi "Cloud Steps" (`KismetMathLibrary.Conv_IntToDouble` (`self.Cloud Steps`)))
  (`MaterialInstanceDynamic.SetScalarParameterValue` _uca_dmi "Atmosphere Light Steps" (`KismetMathLibrary.Conv_IntToDouble` (`self.Atmosphere Light Steps`)))
  (`MaterialInstanceDynamic.SetScalarParameterValue` _uca_dmi "Cloud Light Steps" (`KismetMathLibrary.Conv_IntToDouble` (`self.Cloud Light Steps`)))
  (`MaterialInstanceDynamic.SetScalarParameterValue` _uca_dmi "Step Scale Factor" (`self.Step Scale Factor`))
  ; Post Process
  (`MaterialInstanceDynamic.SetScalarParameterValue` _uca_post "Atmosphere Radius" (+ _x (* _x (`self.Atmosphere Height Scale`))))
  (`MaterialInstanceDynamic.SetScalarParameterValue` _uca_post "Blur Falloff Factor" (`self.Blur Falloff Factor`))
  (`MaterialInstanceDynamic.SetScalarParameterValue` _uca_post "MaxW" (`self.Out Atmosphere Blur`))
  (`MaterialInstanceDynamic.SetScalarParameterValue` _uca_post "MinW" (`self.In Atmosphere Blur`)))

(fn `UserConstructionScript`
  (bind _starlight (`self.StarLight`))
  (bind _returnvalue (`KismetMathLibrary.Conv_LinearColorToVector` (`self.Light Color`)))
  (bind _settings (`PostProcessComponent.Settings` (`self.UCA_PostProcess`)))
  (bind ((`WeightedBlendables` _weightedblendables)) (break `PostProcessSettings` _settings))
  (bind _returnvalue_2 (`KismetMathLibrary.VSize` _returnvalue))
  (bind _array (break `WeightedBlendables` _weightedblendables))
  (bind _returnvalue_3 (`KismetMathLibrary.FMax` (`KismetMathLibrary.FMax` (.x (`self.GetActorRelativeScale3D`)) (.y (`self.GetActorRelativeScale3D`))) (.z (`self.GetActorRelativeScale3D`))))
  ; Create Dynamic Material Instance in Raymarcher/Post Process Slot
  (bind _returnvalue_4 (`KismetMaterialLibrary.CreateDynamicMaterialInstance` "/CloudAtmosphere/Material/MT_UGA_Default_Inst.MT_UGA_Default_Inst"))
  (bind _output_get (set `self.UCA_DMI` _returnvalue_4))
  (bind _returnvalue_5 (`KismetMaterialLibrary.CreateDynamicMaterialInstance` "/CloudAtmosphere/Material/MT_UCA_Postprocess_Inst.MT_UCA_Postprocess_Inst"))
  (bind _output_get_2 (set `self.UCA_POST` _returnvalue_5))
  (`KismetArrayLibrary.Array_Set` _array 1 (make `WeightedBlendable` 1.0 _output_get) true)
  (`KismetArrayLibrary.Array_Set` _array 2 (make `WeightedBlendable` 2.0 _output_get_2) true)
  (setmembers `PostProcessSettings` :`StructRef` _settings :`WeightedBlendables` _weightedblendables)
  ; Dissallow Axis Specific Scaling
  (`self.SetActorRelativeScale3D` (`KismetMathLibrary.MakeVector` _returnvalue_3 _returnvalue_3 _returnvalue_3))
  ; Hook up Materials
  (`self.MaterialHooks`)
  ; Init Directional Light
  (`LightComponent.SetIntensity` _starlight _returnvalue_2)
  (`LightComponent.SetLightColor` _starlight (`KismetMathLibrary.Conv_VectorToLinearColor` (/ _returnvalue _returnvalue_2)) true))